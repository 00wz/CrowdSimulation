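; Blueprint that simulates a crowd of enemies around the ThirdPersonCharacter, drawn by a single Niagara system rather than individual actors.
; BeginPlay scatters positions at random angles and distances around the player and spawns the shadow-casting system.
; Each Tick moves every position along its horizontal player-to-enemy axis by MoveSpeed and recomputes its offset-corrected rotation.
; It then pushes both arrays into Niagara array parameters.
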(event EventBeginPlay
  ;[1 1 1] Spawn
  (bind _returnvalue (Actor|GetActorOfClass "/Game/ThirdPersonBP/Blueprints/ThirdPersonCharacter.ThirdPersonCharacter_C"))
  (bind _output_get (Variables|Default|SetPlayer _returnvalue))
  (for _index (range 1 (Variables|Default|GetEnemyCount))
    (Utilities|Array|Add (Variables|Default|GetPositionsArray) (+ (Transformation|GetActorLocation _output_get) (Math|Vector|RotateVectorAroundAxis (Math|Vector|MakeVector (Math|Random|RandomFloatinRange 7e+02 1e+02) 0.0 0.0) (Math|Random|RandomFloatinRange 0.0 3.6e+02) "0, 0,1.000000")))
    (Utilities|Array|Add (Variables|Default|GetRotationArray) (Utilities|Struct|MakeQuat 0.0 0.0 0.0 1.0)))
  (bind _returnvalue_2 (Niagara|SpawnSystematLocation "/Game/NiagaraSystems/EnemyesNiagaraSystem.EnemyesNiagaraSystem" "0, 0, 0" "0, 0, 0" "1.000000,1.000000,1.000000" false))
  (bind _output_get_2 (Variables|Default|SetNiagaraSystem _returnvalue_2))
  (Rendering|SetCastShadow _output_get_2 true))

(event EventTick
  (params (DeltaSeconds :type Float%20%28single-precision%29))
  (bind _niagarasystem (Variables|Default|GetNiagaraSystem))
  ;[1 1 1] Moving
  (for (_array_element _array_index) (Variables|Default|GetPositionsArray)
    (Utilities|FlowControl|Sequence
      (:then_0
        (Utilities|Array|SetArrayElem (Variables|Default|GetRotationArray) _array_index (* (Math|Conversions|ToQuaternion(Rotator) (Math|Vector|MakeVector (.x (- _array_element (Transformation|GetActorLocation (Variables|Default|GetPlayer)))) (.y (- _array_element (Transformation|GetActorLocation (Variables|Default|GetPlayer)))) 0.0)) (Variables|Default|GetParticleRotationOffset))))
      (:then_1
        (Utilities|Array|SetArrayElem (Variables|Default|GetPositionsArray) _array_index (+ _array_element (* (* (Math|Vector|Normalize (Math|Vector|MakeVector (.x (- _array_element (Transformation|GetActorLocation (Variables|Default|GetPlayer)))) (.y (- _array_element (Transformation|GetActorLocation (Variables|Default|GetPlayer)))) 0.0)) DeltaSeconds) (Variables|Default|GetMoveSpeed)))))))
  (Class|NiagaraDataInterfaceArrayFunctionLibrary|SetNiagaraArrayVector _niagarasystem "InputPositions" (Variables|Default|GetPositionsArray))
  (Class|NiagaraDataInterfaceArrayFunctionLibrary|SetNiagaraArrayQuat _niagarasystem "InputRotations" (Variables|Default|GetRotationArray)))

(fn ConstructionScript
  (|CallParentFunction))