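; Game mode that runs an enemy movement test without crowd simulation, as its name suggests.
; BeginPlay spawns EnemyCount BP_Enemy actors at random angles and distances around the ThirdPersonCharacter and stores them in an array.
; Tick loops over that array, rotating and offsetting each enemy along the flattened player-to-enemy direction, scaled by MoveSpeed and delta time, without sweep.
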(event EventBeginPlay
  ;[1 1 1] Spawn
  (bind _returnvalue (Actor|GetActorOfClass "/Game/ThirdPersonBP/Blueprints/ThirdPersonCharacter.ThirdPersonCharacter_C"))
  (bind _output_get (Variables|Default|SetPlayer _returnvalue))
  (for _index (range 1 (Variables|Default|GetEnemyCount))
    (bind _returnvalue_2 (Game|SpawnActorfromClass "/Game/Blueprints/BP_Enemy.BP_Enemy_C" (Math|Transform|MakeTransform (+ (Transformation|GetActorLocation _output_get) (Math|Vector|RotateVectorAroundAxis (Math|Vector|MakeVector (Math|Random|RandomFloatinRange 7e+02 1e+02) 0.0 0.0) (Math|Random|RandomFloatinRange 0.0 3.6e+02) "0, 0,1.000000")) "0, 0, 0" "1,1,1") "Undefined" 0 0))
    (Utilities|Array|Add (Variables|Default|GetEnemyes) _returnvalue_2)))

(event EventTick
  (params (DeltaSeconds :type Float%20%28single-precision%29))
  ;[1 1 1] Moving
  (for _array_element (Variables|Default|GetEnemyes)
    (Utilities|FlowControl|Sequence
      (:then_0
        (Transformation|SetActorRotation _array_element (Math|Rotator|FindLookatRotation (Math|Vector|MakeVector 0.0 0.0 0.0) (Math|Vector|MakeVector (.x (- (Transformation|GetActorLocation _array_element) (Transformation|GetActorLocation (Variables|Default|GetPlayer)))) (.y (- (Transformation|GetActorLocation _array_element) (Transformation|GetActorLocation (Variables|Default|GetPlayer)))) 0.0))))
      (:then_1
        (Transformation|AddActorWorldOffset _array_element (* (* (Math|Vector|Normalize (Math|Vector|MakeVector (.x (- (Transformation|GetActorLocation _array_element) (Transformation|GetActorLocation (Variables|Default|GetPlayer)))) (.y (- (Transformation|GetActorLocation _array_element) (Transformation|GetActorLocation (Variables|Default|GetPlayer)))) 0.0)) DeltaSeconds) (Variables|Default|GetMoveSpeed)))))))

(fn ConstructionScript
  (|CallParentFunction))